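; Base weapon Blueprint for the SpreadShot game, providing fire-rate gating with empty Fire and StopFiring events.
; BeginPlay converts rounds per second into a seconds-per-shot interval.
; StartFiring calls Fire if that interval has passed since the last shot, otherwise it stores a timer set for the full interval.
; Unconnected nodes sketch a last-shot reset and loops splitting accurate from remaining projectiles.
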(event `Start Firing`
  (bind _firerate_timer (`self.FireRate_Timer`))
  (if (> (- (`KismetSystemLibrary.GetGameTimeInSeconds`) (`self.TimeOfLastShot`)) _firerate_timer)
    (`self.Fire`)
    (else
      (bind _returnvalue (`KismetSystemLibrary.K2_SetTimerDelegate` (`|CreateDelegate` :!event `Fire`) _firerate_timer))
      (set `self.NextShotTimer` _returnvalue))))

(event `Stop Firing`)

(event `Fire`)

(event `self.ReceiveBeginPlay`
  (set `self.FireRate_Timer` (/ 1.0 (`self.FireRate_RPS`))))

(fn `UserConstructionScript`)